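; Interactable laptop actor that the player can use as a full-screen computer interface and then close.
; BeginPlay creates a LaptopScreen widget and assigns it to the in-world ScreenWidget.
; Interact freezes player movement, animates the lid, blends to the laptop camera, then shows the same widget in the viewport with UI-only input.
; CloseLap reverses this, restoring the player's camera, walking and game input; PickupItem only returns zero.
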(event Custom|CloseLap
  (bind _returnvalue (Game|GetPlayerController 0))
  (if (Variables|Default|GetInUse)
    (Widget|RemovefromParent (Variables|Default|GetLaptopWidgetScreen))
    (Components|MoveComponentTo (Variables|Default|GetScreen) (Variables|/Script/Engine.SceneComponent|GetRelativeLocation (Variables|Default|GetScreen)) "0,0.000000,105.000000" true true 1.0 false)
    (Game|Player|SetViewTargetwithBlend _returnvalue (Components|GetOwner (Variables|/Game/ThirdPersonBP/Blueprints/ZE_HeroCharacter.ZE_HeroCharacter_C|GetFollowCamera (stale EventInteract Player))) 0.5 "VTBlend_Linear" 0.0 false)
    (Pawn|Components|CharacterMovement|SetMovementMode (Variables|/Script/Engine.Character|GetCharacterMovement (stale EventInteract Player)) "MOVE_Walking" 0)
    (Variables|Default|SetInUse false)
    (Input|DisableInput _returnvalue)
    (Variables|/Script/Engine.PlayerController|SetbShowMouseCursor _returnvalue false)
    (Default|CloseBinds (Variables|Default|GetLaptopWidgetScreen))
    (Input|SetInputModeGameOnly _returnvalue)))

(event EventInteract
  (params (Player :type ZE%20Hero%20Character%20Object%20Reference))
  (bind _returnvalue (Game|GetPlayerController 0))
  (bind _laptopwidgetscreen (Variables|Default|GetLaptopWidgetScreen))
  (bind _charactermovement (Variables|/Script/Engine.Character|GetCharacterMovement Player))
  (if (not (Variables|Default|GetInUse))
    (Input|EnableInput (Game|GetPlayerController 0))
    (Components|Movement|StopMovementImmediately _charactermovement)
    (Pawn|Components|CharacterMovement|SetMovementMode _charactermovement "MOVE_None" 0)
    (Components|MoveComponentTo (Variables|Default|GetScreen) (Variables|/Script/Engine.SceneComponent|GetRelativeLocation (Variables|Default|GetScreen)) "0, 0, 0" true true 1.0 false)
    (Variables|Default|SetInUse true)
    (Game|Player|SetViewTargetwithBlend _returnvalue (Components|GetOwner (Variables|Default|GetCamera)) 0.5 "VTBlend_Linear" 0.0 true)
    (Input|EnableInput _returnvalue)
    (Variables|/Script/Engine.PlayerController|SetbShowMouseCursor _returnvalue true)
    (Utilities|FlowControl|Delay 0.5)
    (UserInterface|Viewport|AddtoViewport _laptopwidgetscreen 0)
    (Default|BindButtons _laptopwidgetscreen)
    (Input|SetInputModeUIOnly _returnvalue _laptopwidgetscreen "DoNotLock")))

(event EventBeginPlay
  (bind _returnvalue (UserInterface|CreateWidget "/Game/GameBPs/UIofGame/LaptopScreen.LaptopScreen_C"))
  (bind _output_get (Variables|Default|SetLaptopWidgetScreen _returnvalue))
  (UserInterface|SetWidget (Variables|Default|GetScreenWidget) _output_get))

(fn ConstructionScript)

(fn PickupItem
  (params (Player :type ZE%20Hero%20Character%20Object%20Reference))
  (return 0 0))