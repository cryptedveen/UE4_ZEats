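; Interactable radio actor that plays one of four randomly chosen audio components when Interact fires.
; Each Interact adds a new component without stopping the previous one, so key 1 stops only the latest.
; Box overlap toggles player input for any actor, but shows or hides the text prompt only for Hero-tagged actors implementing GameBPI.
; PickupItem is a stub returning zero quantity.
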(event OnComponentBeginOverlap(Box)
  (params (OverlappedComponent :type Primitive%20Component%20Object%20Reference) (OtherActor :type Actor%20Object%20Reference) (OtherComp :type Primitive%20Component%20Object%20Reference) (OtherBodyIndex :type Integer) (bFromSweep :type Boolean) (SweepResult :type Hit%20Result%20Structure%20%28by%20ref%29))
  (Input|EnableInput (Game|GetPlayerController 0))
  (if (and (Actor|ActorHasTag OtherActor "Hero") (Utilities|DoesObjectImplementInterface OtherActor "/Game/GameBPs/BP_Interfaces/GameBPI.GameBPI_C"))
    (Rendering|SetVisibility (Variables|Default|GetTextRender) true false)))

(event OnComponentEndOverlap(Box)
  (params (OverlappedComponent :type Primitive%20Component%20Object%20Reference) (OtherActor :type Actor%20Object%20Reference) (OtherComp :type Primitive%20Component%20Object%20Reference) (OtherBodyIndex :type Integer))
  (Input|DisableInput (Game|GetPlayerController 0))
  (if (and (Actor|ActorHasTag OtherActor "Hero") (Utilities|DoesObjectImplementInterface OtherActor "/Game/GameBPs/BP_Interfaces/GameBPI.GameBPI_C"))
    (Rendering|SetVisibility (Variables|Default|GetTextRender) false false)))

(event EventBeginPlay)

(event EventInteract
  (params (Player :type ZE%20Hero%20Character%20Object%20Reference))
  (switch int (Math|Random|RandomIntegerinRange 0 3)
    (:0
      (bind _returnvalue (AddComponent|AddAudioComponent false))
      (Variables|Default|SetPlayingMusic _returnvalue))
    (:1
      (bind _returnvalue_2 (AddComponent|AddAudioComponent false))
      (Variables|Default|SetPlayingMusic _returnvalue_2))
    (:2
      (bind _returnvalue_3 (AddComponent|AddAudioComponent false))
      (Variables|Default|SetPlayingMusic _returnvalue_3))
    (:3
      (bind _returnvalue_4 (AddComponent|AddAudioComponent false))
      (Variables|Default|SetPlayingMusic _returnvalue_4)))
  (Audio|Components|Audio|Play (Variables|Default|GetPlayingMusic) 0.0))

(event Input|KeyboardEvents|1
  (params (Key :type Key%20Structure :default "None"))
  (:Pressed
    (Audio|Components|Audio|Stop (Variables|Default|GetPlayingMusic))))

(fn ConstructionScript)

(fn PickupItem
  (params (Player :type ZE%20Hero%20Character%20Object%20Reference))
  (return 0 0))