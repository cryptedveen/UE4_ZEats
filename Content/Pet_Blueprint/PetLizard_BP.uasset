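; Lizard pet Blueprint that wanders around its surroundings and plays an eating animation when interacted with.
; A self-repeating roam event sends AI moves to random reachable nearby points, re-issuing after a random delay from each request rather than waiting for arrival.
; Interact stops movement immediately and plays the eat montage, but leaves the roam loop running.
; PickupItem is a stub returning zero quantity.
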(event Custom|LizardRoam
  (AI|AIMoveTo self (.RandomLocation (AI|Navigation|GetRandomReachablePointinRadius (Transformation|GetWorldLocation (Variables|Collision|GetCapsuleComponent)) 1e+02 0 0)) 0 1.0 false
    (:then
      (Utilities|FlowControl|Delay (Math|Random|RandomFloatinRange 1.0 3.0))
      (CallFunction|LizardRoam))))

(event EventBeginPlay
  (CallFunction|LizardRoam))

(event EventInteract
  (params (Player :type ZE%20Hero%20Character%20Object%20Reference))
  (Components|Movement|StopMovementImmediately (Variables|Character|GetCharacterMovement))
  (bind _returnvalue (Animation|PlayAnimMontage "/Game/Pet_Blueprint/Animations/EatMontage.EatMontage" 1.0 "None"))
  (Utilities|FlowControl|Delay _returnvalue))

(fn ConstructionScript)

(fn PickupItem
  (params (Player :type ZE%20Hero%20Character%20Object%20Reference))
  (return 0 0))